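; EditableObject is a clickable actor that the player's BP_EditorChar can select for in-game editing.
; Its construction script applies one Mesh variable to both the Object component and a Highlight component, which shows only while the cursor hovers.
; Clicks alternate through a FlipFlop, swapping the highlight between frame and disc materials and telling the character to begin or end editing.
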(event `self.ReceiveActorBeginCursorOver`
  (`SceneComponent.SetVisibility` (`self.Highlight`) true false))

(event `self.ReceiveActorEndCursorOver`
  (`SceneComponent.SetVisibility` (`self.Highlight`) false false))

(event `self.ReceiveActorOnClicked`
  (params (ButtonPressed :type "Key Structure"))
  (`/Engine/EditorBlueprintResources/StandardMacros.FlipFlop`
    (:`A`
      (`PrimitiveComponent.SetMaterial` (`self.Highlight`) 0 "/Engine/VREditor/UI/FrameMaterial.FrameMaterial")
      (bind _asbp_editor_char (cast `/Game/PlayerCharacter/EditMode/BP_EditorChar` (`GameplayStatics.GetPlayerCharacter` 0)))
      (`/Game/PlayerCharacter/EditMode/BP_EditorChar.BeginEditObject` _asbp_editor_char self))
    (:`B`
      (`PrimitiveComponent.SetMaterial` (`self.Highlight`) 0 "/Engine/VREditor/UI/DiscMaterial.DiscMaterial")
      (bind _asbp_editor_char_2 (cast `/Game/PlayerCharacter/EditMode/BP_EditorChar` (`GameplayStatics.GetPlayerCharacter` 0)))
      (`/Game/PlayerCharacter/EditMode/BP_EditorChar.EndEditObject` _asbp_editor_char_2))))

(fn `UserConstructionScript`
  (bind _mesh (`self.Mesh`))
  (`StaticMeshComponent.SetStaticMesh` (`self.Highlight`) _mesh)
  (`StaticMeshComponent.SetStaticMesh` (`self.Object`) _mesh))